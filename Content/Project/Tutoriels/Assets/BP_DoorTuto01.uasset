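; BP_DoorTuto01 is a padlocked tutorial door that opens for the tagged player once they have the key.
; On overlap, the hidden key appears and a timeline animates it, then, after a delay, key and lock drop with physics.
; This clears PlayerHasKey on KeyRef and sets DoorUnlocked, letting a second timeline swing the door open.
; Later player overlaps reopen the unlocked door, and ending any overlap reverses the swing.
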(event OnComponentBeginOverlap(CollisionBox)
  (params (OverlappedComponent :type Primitive%20Component%20Object%20Reference) (OtherActor :type Actor%20Object%20Reference) (OtherComp :type Primitive%20Component%20Object%20Reference) (OtherBodyIndex :type Integer) (bFromSweep :type Boolean) (SweepResult :type Hit%20Result%20Structure%20%28by%20ref%29))
  (bind _key (Variables|Default|GetKey))
  (bind _key_2 (Variables|Default|GetKey))
  (bind _lock (Variables|Default|GetLock))
  (if (Actor|ActorHasTag OtherActor "Joueur")
    (Utilities|FlowControl|Sequence
      (:then_0
        (if (Variables|/Game/Project/Tutoriels/Assets/BP_KeyTuto01.BP_KeyTuto01_C|GetPlayerHasKey (Variables|Default|GetKeyRef))
          (if (not (Variables|Default|GetDoorUnlocked))
            (Rendering|SetVisibility _key true false)
            (Collision|SetCollisionEnabled _key "QueryAndPhysics")
            (Utilities|FlowControl|Delay 0.5)
            (bind (_direction _keyfirstanim _newtrack_3) (Timeline|KeyTimeline Play)
              (:Update
                ;[0.15 0.15 0.15 0.5] Première animation de clé
                (Transformation|SetRelativeLocation _key _keyfirstanim false false)
                ;[0.15 0.15 0.15 0.5] Deuxième animation de clé
                (Transformation|SetRelativeRotation _key_2 (Math|Rotator|MakeRotator 0.0 (Math|Float|Lerp 9e+01 0.0 _newtrack_3) 9e+01) false false)
                (Utilities|FlowControl|Delay 3.0)
                ;[0.15 0.15 0.15 0.5] Faire tomber le cadenas et la clé et ajuster leurs collisions pour éviter des bugs
                (Physics|SetSimulatePhysics _key_2 true)
                (Collision|SetCollisionEnabled _key_2 "PhysicsOnly")
                (Physics|SetSimulatePhysics _lock true)
                (Collision|SetCollisionEnabled _lock "PhysicsOnly")
                ;[0.15 0.15 0.15 0.5] on la remet à false pour éviter bugs
                (Variables|/Game/Project/Tutoriels/Assets/BP_KeyTuto01.BP_KeyTuto01_C|SetPlayerHasKey (Variables|Default|GetKeyRef) false)
                (Variables|Default|SetDoorUnlocked true)
                (if (Variables|Default|GetDoorUnlocked) :!label _label
                  (bind _newtrack_0 (Timeline|Timeline Play)
                    (:Update
                      (Transformation|SetRelativeRotation (Variables|Default|GetDoor) (Math|Rotator|MakeRotator 0.0 0.0 (Math|Float|Lerp 0.0 9e+01 _newtrack_0)) false false)))))))))
      (:then_1
        (goto _label)))))

(event OnComponentEndOverlap(CollisionBox)
  (params (OverlappedComponent :type Primitive%20Component%20Object%20Reference) (OtherActor :type Actor%20Object%20Reference) (OtherComp :type Primitive%20Component%20Object%20Reference) (OtherBodyIndex :type Integer))
  (bind _newtrack_0 (Timeline|Timeline Reverse)
    (:Update
      (Transformation|SetRelativeRotation (Variables|Default|GetDoor) (Math|Rotator|MakeRotator 0.0 0.0 (Math|Float|Lerp 0.0 9e+01 _newtrack_0)) false false))))

(event EventBeginPlay
  (bind _key (Variables|Default|GetKey))
  ;[0.15 0.15 0.15 0.5] On cache la clé dès le début
  (Rendering|SetVisibility _key false false)
  (Collision|SetCollisionEnabled _key "NoCollision"))

(fn ConstructionScript)