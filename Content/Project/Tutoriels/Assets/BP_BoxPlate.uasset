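; BP_BoxPlate is a pressure plate that opens a linked door when the player or a specific tagged box overlaps its trigger box.
; Overlap events call OpenDoor and CloseDoor on DoorRef, with the BoxTag variable pairing a particular box to a particular door.
; A BoxIn flag keeps the door open when the player steps off while the box remains, but removing the box always closes it.
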(event OnComponentBeginOverlap(Box)
  (params (OverlappedComponent :type Primitive%20Component%20Object%20Reference) (OtherActor :type Actor%20Object%20Reference) (OtherComp :type Primitive%20Component%20Object%20Reference) (OtherBodyIndex :type Integer) (bFromSweep :type Boolean) (SweepResult :type Hit%20Result%20Structure%20%28by%20ref%29))
  (Utilities|FlowControl|Sequence
    (:then_0
      (if (Actor|ActorHasTag OtherActor "Joueur")
        (Default|OpenDoor (Variables|Default|GetDoorRef) :!label _label)))
    (:then_1
      (if (Actor|ActorHasTag OtherActor (Variables|Default|GetBoxTag))
        (Variables|Default|SetBoxIn? true)
        (goto _label)))))

(event OnComponentEndOverlap(Box)
  (params (OverlappedComponent :type Primitive%20Component%20Object%20Reference) (OtherActor :type Actor%20Object%20Reference) (OtherComp :type Primitive%20Component%20Object%20Reference) (OtherBodyIndex :type Integer))
  (Utilities|FlowControl|Sequence
    (:then_0
      (if (Actor|ActorHasTag OtherActor (Variables|Default|GetBoxTag))
        (Variables|Default|SetBoxIn? false)
        (Default|CloseDoor (Variables|Default|GetDoorRef) :!label _label)))
    (:then_1
      (if (Actor|ActorHasTag OtherActor "Joueur")
        (if (not (Variables|Default|GetBoxIn?))
          (goto _label))))))

(fn ConstructionScript)