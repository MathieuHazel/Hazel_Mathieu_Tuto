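; Tutorial door Blueprint that stays locked until the player has picked up its key.
; On Interact with the key, a hidden key mesh appears and animates through a Timeline, then after delays key and lock fall under physics and a light turns green.
; Once unlocked, further interactions alternately open and close the door through a FlipFlop driving a rotation Timeline.
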(event EventPickUpKey
  (Variables|Default|SetPickedUp? true))

(event EventInteract
  (bind _key (Variables|Default|GetKey))
  (bind _key_2 (Variables|Default|GetKey))
  (bind _lock (Variables|Default|GetLock))
  (if (Variables|Default|GetPickedUp?)
    (Utilities|FlowControl|Sequence
      (:then_0
        (if (not (Variables|Default|GetUnlocked?))
          (Rendering|SetVisibility _key true false)
          (Collision|SetCollisionEnabled _key "QueryAndPhysics")
          (Utilities|FlowControl|Delay 0.5)
          ;[0.15 0.15 0.15 0.5] Première animation de clé
          (bind (_direction _keyfirstanim _newtrack_3) (Timeline|Timeline Play)
            (:Update
              (Transformation|SetRelativeLocation _key _keyfirstanim false false)
              ;[0.15 0.15 0.15 0.5] Deuxième animation de clé
              (Transformation|SetRelativeRotation _key_2 (Math|Rotator|MakeRotator 0.0 (Math|Float|Lerp 9e+01 0.0 _newtrack_3) 9e+01) false false)
              (Utilities|FlowControl|Delay 3.0)
              ;[0.15 0.15 0.15 0.5] Faire tomber le cadenas et la clé et ajuster leurs collisions pour éviter des bugs
              (Physics|SetSimulatePhysics _key_2 true)
              (Collision|SetCollisionEnabled _key_2 "PhysicsOnly")
              (Physics|SetSimulatePhysics _lock true)
              (Collision|SetCollisionEnabled _lock "PhysicsOnly")
              (Variables|Default|SetUnlocked? true)
              (Rendering|Material|SetMaterial (Variables|Default|GetActualLight) 0 "/Game/Project/Tutoriels/Materials/M_Green_Shiny.M_Green_Shiny")))))
      (:then_1
        (if (Variables|Default|GetUnlocked?)
          (Utilities|FlowControl|FlipFlop
            (:A
              (bind _newtrack_0 (Timeline|TimelineDoor Play)
                (:Update
                  (Transformation|SetRelativeRotation (Variables|Default|GetDoor) (Math|Rotator|MakeRotator 0.0 0.0 (Math|Float|Lerp 0.0 9e+01 _newtrack_0)) false false))))
            (:B
              (Timeline|TimelineDoor Reverse))))))))

(event EventBeginPlay
  (bind _key (Variables|Default|GetKey))
  ;[0.15 0.15 0.15 0.5] On cache la clé dès le début
  (Rendering|SetVisibility _key false false)
  (Collision|SetCollisionEnabled _key "NoCollision"))

(fn ConstructionScript)