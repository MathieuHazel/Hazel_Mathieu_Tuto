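; Tutorial door that stays locked until its pickup event marks the key as collected.
; The first interaction reveals the hidden key and animates its position and rotation with a timeline.
; After a delay, key and lock switch to physics, the door unlocks and the indicator material turns green.
; Later interactions use a FlipFlop to play or reverse a timeline that swings the door 90 degrees.
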(event EventPickUpKey
  (Variables|Default|SetPickedUp? true))

(event EventInteract
  (bind _key (Variables|Default|GetKey))
  (bind _key_2 (Variables|Default|GetKey))
  (bind _key_3 (Variables|Default|GetKey))
  (bind _lock (Variables|Default|GetLock))
  (if (Variables|Default|GetPickedUp?)
    (Utilities|FlowControl|Sequence
      (:then_0
        (if (not (Variables|Default|GetUnlocked?))
          (Rendering|SetVisibility _key_2 true false)
          (Collision|SetCollisionEnabled _key_2 "QueryAndPhysics")
          (Utilities|FlowControl|Delay 0.5)
          (bind (_direction _animation1 _animation2) (Timeline|Timeline Play)
            (:Update
              (Transformation|SetRelativeLocation _key _animation1 false false)
              (Transformation|SetRelativeRotation _key (Math|Rotator|MakeRotator 0.0 (Math|Float|Lerp 9e+01 0.0 _animation2) 9e+01) false false)
              (Utilities|FlowControl|Delay 3.0)
              (Physics|SetSimulatePhysics _key_3 true)
              (Collision|SetCollisionEnabled _key_3 "PhysicsOnly")
              (Physics|SetSimulatePhysics _lock true)
              (Collision|SetCollisionEnabled _lock "PhysicsOnly")
              (Variables|Default|SetUnlocked? true)
              (Rendering|Material|SetMaterial (Variables|Default|GetActualLight) 0 "/Game/Project/Tutoriels/Materials/M_Green_Shiny.M_Green_Shiny")))))
      (:then_1
        (if (Variables|Default|GetUnlocked?)
          (Utilities|FlowControl|FlipFlop
            (:A
              (bind _newtrack_0 (Timeline|Timeline_0 Play)
                (:Update
                  (Transformation|SetRelativeRotation (Variables|Default|GetDoor) (Math|Rotator|MakeRotator 0.0 0.0 (Math|Float|Lerp 0.0 9e+01 _newtrack_0)) false false))))
            (:B
              (Timeline|Timeline_0 Reverse))))))))

(event EventBeginPlay
  (bind _key (Variables|Default|GetKey))
  (Rendering|SetVisibility _key false false)
  (Collision|SetCollisionEnabled _key "NoCollision"))

(fn ConstructionScript)