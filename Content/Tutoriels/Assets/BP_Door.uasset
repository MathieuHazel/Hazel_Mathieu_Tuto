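; BP_Door is a tutorial door that swings open for a player carrying a key.
; When an actor tagged "Joueur" enters the Box trigger and KeyRef reports the key, a timeline plays and lerps the Door's relative yaw to a quarter turn.
; Any actor leaving the Box reverses the timeline, without tag or key checks.
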(event OnComponentBeginOverlap(Box)
  (params (OverlappedComponent :type Primitive%20Component%20Object%20Reference) (OtherActor :type Actor%20Object%20Reference) (OtherComp :type Primitive%20Component%20Object%20Reference) (OtherBodyIndex :type Integer) (bFromSweep :type Boolean) (SweepResult :type Hit%20Result%20Structure%20%28by%20ref%29))
  (if (Actor|ActorHasTag OtherActor "Joueur")
    (if (Variables|/Game/Tutoriels/Assets/BP_Key.BP_Key_C|GetPlayerHasKey (Variables|Default|GetKeyRef))
      (bind _nouvelle_piste_0 (Timeline|Chronologie Play)
        (:Update
          (Transformation|SetRelativeRotation (Variables|Default|GetDoor) (Math|Rotator|MakeRotator 0.0 0.0 (Math|Float|Lerp 0.0 9e+01 _nouvelle_piste_0)) false false))))))

(event OnComponentEndOverlap(Box)
  (params (OverlappedComponent :type Primitive%20Component%20Object%20Reference) (OtherActor :type Actor%20Object%20Reference) (OtherComp :type Primitive%20Component%20Object%20Reference) (OtherBodyIndex :type Integer))
  (bind _nouvelle_piste_0 (Timeline|Chronologie Reverse)
    (:Update
      (Transformation|SetRelativeRotation (Variables|Default|GetDoor) (Math|Rotator|MakeRotator 0.0 0.0 (Math|Float|Lerp 0.0 9e+01 _nouvelle_piste_0)) false false))))

(fn ConstructionScript)